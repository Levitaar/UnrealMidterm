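; PlayerBP is a player Blueprint that provides basic input-driven movement and turning.
; The RL and FB axis inputs offset the actor along its right and forward vectors with swept SetActorLocation calls.
; MouseX adds scaled yaw to the actor's rotation, which also steers the movement directions.
; Steps are fixed multiples of the axis value, with no delta-time scaling or movement component calls.
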(event Input|AxisEvents|InputAxisFB
  (params (AxisValue :type Float%20%28single-precision%29))
  (Transformation|SetActorLocation (+ (* (Transformation|GetActorForwardVector) (* AxisValue 1e+01)) (Transformation|GetActorLocation)) true false))

(event Input|AxisEvents|InputAxisRL
  (params (AxisValue :type Float%20%28single-precision%29))
  (Transformation|SetActorLocation (+ (* (Transformation|GetActorRightVector) (* AxisValue 1e+01)) (Transformation|GetActorLocation)) true false))

(event Input|MouseEvents|MouseX
  (params (AxisValue :type Float%20%28single-precision%29))
  (Transformation|SetActorRotation (Math|Rotator|CombineRotators (Transformation|GetActorRotation) (Math|Rotator|MakeRotator 0.0 0.0 (* AxisValue 5.0)))))

(fn ConstructionScript)